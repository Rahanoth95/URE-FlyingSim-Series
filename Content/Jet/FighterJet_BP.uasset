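; Player-controlled fighter jet pawn that taxis, takes off, flies and lands, with a HUD created on BeginPlay.
; A Flying flag switches inputs between ground steering with free camera and pitch, yaw, roll and throttle, while setting wheel and control-surface rotations.
; Tick moves the jet along its forward vector using interpolated thrust, which also scales exhaust effects.
; A downward trace each flying tick lands and levels the jet when target thrust is low.
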(event EventBeginPlay
  ;[1 1 1] Start
  (Utilities|FlowControl|Sequence
    (:then_0
      (Variables|Speed|SetTarget%20Thrust%20Speed (Variables|Speed|GetMinimum%20Thrust%20Speed))
      ;;[1 1 1] Setting offset for landing
      (Variables|Default|SetStart%20Z%20Offset 131.0)
      ;;[1 1 1] Create & Add Hud
      (bind _returnvalue (UserInterface|CreateWidget "/Game/Jet/HUD/Jet_UI.Jet_UI_C"))
      (bind _output_get (Variables|Default|SetHUD%20Ref _returnvalue))
      (UserInterface|Viewport|AddtoViewport _output_get 0))
    (:then_1
      ;;[1 1 1] Set Scale of exhaust partic
      (Transformation|SetRelativeScale3D (Variables|Default|GetLeftExhaust) "0, 0, 0"))))

(event EventTick
  (params (DeltaSeconds :type Float%20%28single-precision%29))
  (bind _current_thrust_speed (Variables|Speed|GetCurrent%20Thrust%20Speed))
  (bind _maximum_thrust_speed (Variables|Speed|GetMaximum%20Thrust%20Speed))
  (bind _returnvalue (Math|Float|NormalizetoRange _current_thrust_speed 0.0 _maximum_thrust_speed))
  ;[1 1 1] Event Tick
  (Utilities|FlowControl|Sequence
    (:then_0
      (bind _output_get (Variables|Default|SetMove%20Forward%20Interp (Math|Float|Clamp(Float) (Math|Interpolation|FInterpTo (stale _output_get) (Input|AxisValues|GetMoveForward) (Utilities|Time|GetWorldDeltaSeconds) 0.2))))
      ;;[1 1 1] Exhaust particle Scale relative
      (Transformation|SetRelativeScale3D (Variables|Default|GetLeftExhaust) (Math|Interpolation|VInterpTo (Variables|/Script/Engine.SceneComponent|GetRelativeScale3D (Variables|Default|GetRightExhaust)) (Math|Vector|SelectVector (Math|Vector|MakeVector _returnvalue _returnvalue _returnvalue) "0, 0, 0" (Variables|Default|GetFlying?)) (Utilities|Time|GetWorldDeltaSeconds) (Math|Float|SelectFloat 4.0 0.5 (Variables|Default|GetFlying?)))))
    (:then_1
      ;;[1 1 1] If Flying
      (if (Variables|Default|GetFlying?)
        (CallFunction|AddFlightMovement)
        (CallFunction|LandingTrace "ForOneFrame" (Variables|Default|GetStart%20Z%20Offset))))))

(event Input|AxisEvents|InputAxisMoveForward
  (params (AxisValue :type Float%20%28single-precision%29))
  (bind _wheel_rotation_side_max (Variables|MeshTransforms|GetWheel%20Rotation%20Side%20Max))
  ;[0.1458 0.7784 1] If flyig, Move forward increase/decrea if not add movement
  (if (Variables|Default|GetFlying?)
    (Variables|Speed|SetTarget%20Thrust%20Speed (Math|Float|Clamp(Float) (+ (* AxisValue (Utilities|Time|GetWorldDeltaSeconds) 1.5e+03) (Variables|Speed|GetTarget%20Thrust%20Speed)) (Variables|Speed|GetMinimum%20Thrust%20Speed) (Variables|Speed|GetMaximum%20Thrust%20Speed))))
  (if (not (Variables|Default|GetFlying?))
    (Utilities|FlowControl|Sequence
      (:then_0
        ;[0.1458 0.7784 1] Slowly Move Plane Across ground, with speed getting higher the longer move forward is insta, Z is zero-d since move up and down only on ground
        (Transformation|AddActorWorldOffset (Math|Vector|MakeVector (.X (Math|Vector|BreakVector (* (Transformation|GetActorForwardVector) (Variables|Default|GetMove%20Forward%20Interp) (/ (Variables|Speed|GetTarget%20Thrust%20Speed) 5e+02)))) (.Y (Math|Vector|BreakVector (* (Transformation|GetActorForwardVector) (Variables|Default|GetMove%20Forward%20Interp) (/ (Variables|Speed|GetTarget%20Thrust%20Speed) 5e+02)))) 0.0))
        ;[0.1458 0.7784 1] If is moving faste enough on ground and space is presssed, plan will beging to fly, Lag is turned on for spring arm for smoother camera flight controls and offset
        (if (and (> (Variables|Default|GetMove%20Forward%20Interp) 0.7) (Game|Player|IsInputKeyDown (Game|GetPlayerController 0) "SpaceBar"))
          (Variables|Default|SetFlying? true)
          (Variables|/Script/Engine.SpringArmComponent|SetbUsePawnControlRotation (Variables|Default|GetSpringArm) false)
          (Transformation|AddActorWorldOffset "0, 0,25.000000" true)))
      (:then_1
        ;[1 0.9177 0.02034] Set Wheel Rotation for side and directional
        (Variables|MeshTransforms|SetWheel%20Rotation (Math|Rotator|MakeRotator 0.0 (+ (.pitch (Transformation|GetSocketRotation (Variables|Default|GetSK_West_Fighter_Typhoon) "front_wheel_jnt")) (* (Variables|Default|GetMove%20Forward%20Interp) -5e+02)) (Math|Interpolation|FInterpTo (.yaw (Variables|MeshTransforms|GetWheel%20Rotation)) (Math|Float|MapRangeClamped (Input|AxisValues|GetMoveRight) -1.0 1.0 (* _wheel_rotation_side_max -1.0) _wheel_rotation_side_max) (Utilities|Time|GetWorldDeltaSeconds) 0.4)))))))

(event Input|AxisEvents|InputAxisMoveRight
  (params (AxisValue :type Float%20%28single-precision%29))
  (bind _aileon_interior_rotation__max (Variables|MeshTransforms|GetAileon%20Interior%20Rotation%20%20Max))
  (bind _aileon_interior_rotation__max_2 (Variables|MeshTransforms|GetAileon%20Interior%20Rotation%20%20Max))
  ;[0.1573 0.8802 1] Move Right Input, if not flying then move on ground as well. if not then A and D keys will rotate the plane on its side
  (if (Variables|Default|GetFlying?)
    (bind _output_get (Variables|PlaneRotation|SetFlight%20Roll (Math|Interpolation|FInterpTo (stale _output_get) AxisValue (Utilities|Time|GetWorldDeltaSeconds) 1e+01)))
    (Transformation|AddActorLocalRotation (Math|Rotator|MakeRotator (* _output_get (Utilities|Time|GetWorldDeltaSeconds) 9e+01) 0.0 0.0) false false)
    (Variables|MeshTransforms|SetAileron%20Flap%20Rotation%20Left (Math|Rotator|MakeRotator 0.0 (Math|Float|MapRangeClamped (Input|AxisValues|GetMoveRight) -1.0 1.0 _aileon_interior_rotation__max_2 (* _aileon_interior_rotation__max_2 -1.0)) 0.0))
    (Variables|MeshTransforms|SetAileron%20Flap%20Rotation%20Right (Math|Rotator|MakeRotator 0.0 (Math|Float|MapRangeClamped (Input|AxisValues|GetMoveRight) -1.0 1.0 (* _aileon_interior_rotation__max -1.0) _aileon_interior_rotation__max) 0.0))
    (else
      ;;[1 1 1] Can only move right/left on ground if moving forward
      (if (> (Input|AxisValues|GetMoveForward) 0.0)
        (Class|Actor|AddActorWorldRotation (Math|Rotator|MakeRotator 0.0 0.0 (* AxisValue (Utilities|Time|GetWorldDeltaSeconds) 1.2)))))))

(event Input|AxisEvents|InputAxisLookUp
  (params (AxisValue :type Float%20%28single-precision%29))
  (bind _returnvalue (Utilities|Time|GetWorldDeltaSeconds))
  (bind _invert_vertical_flight_ (Variables|Default|GetInvert%20Vertical%20Flight?))
  (bind _aileon_interior_rotation__max (Variables|MeshTransforms|GetAileon%20Interior%20Rotation%20%20Max))
  (bind _returnvalue_2 (Math|Float|SelectFloat -1.0 1.0 _invert_vertical_flight_))
  (bind _returnvalue_3 (* AxisValue _returnvalue_2))
  ;[0.1458 0.7784 1] Look up Input. If not flying then add camera rotation if not add rotation to plane
  (if (Variables|Default|GetFlying?)
    (bind _output_get (Variables|PlaneRotation|SetFlight%20Pitch (Math|Interpolation|FInterpTo (stale _output_get) _returnvalue_3 _returnvalue 1e+01)))
    (Transformation|AddActorLocalRotation (Math|Rotator|MakeRotator 0.0 (* _output_get _returnvalue (Variables|PlaneRotation|GetFlight%20Turn%20Rate)) 0.0) false false)
    (Variables|MeshTransforms|SetAileron%20Interior%20Rotation (Math|Rotator|MakeRotator 0.0 (Math|Float|MapRangeClamped (Variables|PlaneRotation|GetFlight%20Pitch) -1.0 1.0 _aileon_interior_rotation__max (* _aileon_interior_rotation__max -1.0)) 0.0))
    (else
      (Pawn|Input|AddControllerPitchInput _returnvalue_3))))

(event Input|AxisEvents|InputAxisTurn
  (params (AxisValue :type Float%20%28single-precision%29))
  (bind _returnvalue (Utilities|Time|GetWorldDeltaSeconds))
  (bind _rudder_rotation_max (Variables|MeshTransforms|GetRudder%20Rotation%20Max))
  ;[0.1458 0.7784 1] Look up Input. If not flying then add camera rotation if not add rotation to plane
  (if (Variables|Default|GetFlying?)
    (bind _output_get (Variables|PlaneRotation|SetFlight%20Turn (Math|Interpolation|FInterpTo (stale _output_get) AxisValue _returnvalue 1e+01)))
    (Transformation|AddActorLocalRotation (Math|Rotator|MakeRotator 0.0 0.0 (* _output_get _returnvalue (Variables|PlaneRotation|GetFlight%20Turn%20Rate))) false false)
    (Variables|MeshTransforms|SetBack%20Rudder%20Rotation (Math|Rotator|MakeRotator 0.0 0.0 (Math|Float|MapRangeClamped (Variables|PlaneRotation|GetFlight%20Turn) -1.0 1.0 _rudder_rotation_max (* _rudder_rotation_max -1.0))))
    (else
      (Pawn|Input|AddControllerYawInput AxisValue))))

(fn ConstructionScript)

(fn AddFlightMovement
  (bind _returnvalue (Utilities|Time|GetWorldDeltaSeconds))
  ;[1 1 1] Set Fligth Speed
  (bind _output_get (Variables|Speed|SetCurrent%20Thrust%20Speed (Math|Interpolation|FInterpTo (stale _output_get) (Variables|Speed|GetTarget%20Thrust%20Speed) _returnvalue 8.0)))
  ;;[1 1 1] Add Movement In forward Direction
  (Transformation|AddActorWorldOffset (* (Math|Vector|GetForwardVector (Variables|Default|GetSK_West_Fighter_Typhoon)) (* _output_get _returnvalue)) true))

(fn FlightMode
  (Variables|Speed|SetCurrent%20Thrust%20Speed 0.0))

(fn LandingTrace
  (params (Debug :type EDrawDebugTrace%20Enum :default "None") (Spawned%20z%20Offset :type Float%20%28double-precision%29))
  (bind _returnvalue (Transformation|GetActorLocation))
  ;[1 1 1] Do line trace from plane Center to position under wheel.
  (bind (_outhit _returnvalue_2) (Collision|LineTraceByChannel _returnvalue (- _returnvalue (Math|Vector|MakeVector 0.0 0.0 Spawned%20z%20Offset)) "TraceTypeQuery1" false (Utilities|Array|MakeArray self) Debug))
  ;[1 1 1] Can only land if Speed is low enough(Controlled by holding W and S)
  (if _returnvalue_2
    (if (< (Math|Float|MapRangeClamped (Variables|Speed|GetTarget%20Thrust%20Speed) (Variables|Speed|GetMinimum%20Thrust%20Speed) (Variables|Speed|GetMaximum%20Thrust%20Speed) 0.0 1.0) 0.5)
      ;[1 1 1] Align plane with floor(Custom Var instead of norms). Rotation is only retained in yaw. Location Set to include height of wheels offset.
      (Variables|Default|SetFlying? false)
      (Transformation|SetActorRelativeTransform (Math|Transform|MakeTransform (Math|Interpolation|VInterpTo (Transformation|GetActorLocation) (+ (.TraceEnd (Collision|BreakHitResult _outhit)) (Math|Vector|MakeVector 0.0 0.0 Spawned%20z%20Offset)) (Utilities|Time|GetWorldDeltaSeconds) 3.0) (Math|Rotator|MakeRotator 0.0 0.0 (.yaw (Transformation|GetActorRotation))) "1.000000,1.000000,1.000000") false false)
      ;[1 1 1] Set Var
      (Variables|/Script/Engine.SpringArmComponent|SetbUsePawnControlRotation (Variables|Default|GetSpringArm) true)
      (Variables|Default|SetMove%20Forward%20Interp 0.0))))

(fn SetCameraLag
  (bind _springarm (Variables|Default|GetSpringArm))
  (bind _flying_ (Variables|Default|GetFlying?))
  (bind _returnvalue (Math|Float|SelectFloat 1e+01 1e+03 _flying_))
  ;[1 1 1] If not flying then lag should be high enough to not be recogn since it is still required for smooth camera to return landing
  (Variables|/Script/Engine.SpringArmComponent|SetCameraLagSpeed _springarm _returnvalue)
  (Variables|/Script/Engine.SpringArmComponent|SetCameraRotationLagSpeed _springarm _returnvalue))